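; Destructible team UAV plane that enemy players shoot down for score.
; On spawn the server assigns its team and a random yaw; enemy damage wakes net dormancy and feeds AC_Health.
; Death awards score, notifies GameState and multicasts an explosion, while the Destroyed RepNotify enables physics and a timed lifespan.
; The wreck tilts on Tick, and the health component's death event loops randomly timed and scaled secondary explosions.
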(event `self.ReceiveAnyDamage`
  (params (Damage :type "Float (single-precision)") (DamageType :type "DamageType Object Reference") (InstigatedBy :type "Controller Object Reference") (DamageCauser :type "Actor Object Reference"))
  (bind _ac_health (`self.AC_Health`))
  (bind _playerstate (`Controller.PlayerState` InstigatedBy))
  ;[0 0 0] Any Damage
  (if (!= (`self.GetTeam` (`self.GetComponentByClass` _playerstate null)) (`self.Team`))
    (if (not (`self.bDestroyed`))
      (message `/Game/Apuroop_FPS_TPS/Blueprints/UAV/BP_UAV_Plane.ShowHitMarker` (`Controller.K2_GetPawn` InstigatedBy) false)
      (`self.SetNetDormancy` "DORM_Awake")
      (`self.HandleDamage` _ac_health Damage)
      (if (`self.IsDead` _ac_health)
        (message `/Game/Apuroop_FPS_TPS/Blueprints/UAV/BP_UAV_Plane.AddScoreToPlayer` _playerstate 350.0 0)
        (`self.OnUAV_Destroyed` (`self.GetComponentByClass` (`GameplayStatics.GetGameState`) null))
        (`self.SetNetDormancy` "DORM_Awake")
        (`self.Explode`)
        (`self.ForceNetUpdate`)))))

(event `Multicast_PlayCostmeticEffects`
  (bind _returnvalue (`SceneComponent.K2_GetComponentLocation` (`self.StaticMesh`)))
  ;[0 0 0] PlayCosmeticEvents
  (`/Engine/EditorBlueprintResources/StandardMacros.Can Execute Cosmetic Events`
    (:`True`
      (`GameplayStatics.SpawnEmitterAtLocation` null _returnvalue (struct) (30.0 30.0 30.0))
      (`GameplayStatics.PlaySoundAtLocation` null _returnvalue (struct) 0.5 1.0 0.0 null null null null))))

(event `Explode`
  ;[0 0 0] Explode
  (`KismetSystemLibrary.Delay` 0.0) ; Next Frame
  (set `self.bDestroyed` true)
  (`self.Multicast_PlayCostmeticEffects`)
  (message `/Game/Apuroop_FPS_TPS/Blueprints/UAV/BP_UAV_Plane.SendMessageToAll` (`GameplayStatics.GetGameState`) "UAV DESTROYED" true))

(event `self.AC_Health.OnPlayerDead`
  (bind _returnvalue (`KismetMathLibrary.RandomFloatInRange` 4.0 18.0))
  (bind _returnvalue_2 (`SceneComponent.K2_GetComponentLocation` (`self.StaticMesh`)))
  ;[0 0 0] On UAV Destroyed
  (`KismetSystemLibrary.Delay` (`KismetMathLibrary.RandomFloatInRange` 0.5 3.0) :!label _label)
  (`GameplayStatics.SpawnEmitterAtLocation` null _returnvalue_2 (struct) (`KismetMathLibrary.MakeVector` _returnvalue _returnvalue _returnvalue))
  (`GameplayStatics.PlaySoundAtLocation` null _returnvalue_2 (struct) 0.5 1.0 0.0 null null null null)
  (goto _label))

(event `self.ReceiveTick`
  (params (DeltaSeconds :type "Float (single-precision)"))
  (bind _staticmesh (`self.StaticMesh`))
  (bind (_relativerotation_roll _relativerotation_pitch _relativerotation_yaw) (`KismetMathLibrary.BreakRotator` (`SceneComponent.RelativeRotation` _staticmesh)))
  ;[0 0 0] Tick
  (if (`self.bDestroyed`)
    (`SceneComponent.K2_SetRelativeRotation` _staticmesh (`KismetMathLibrary.MakeRotator` (+ _relativerotation_roll -0.1) (+ _relativerotation_pitch 0.1) _relativerotation_yaw) false false)))

(event `self.ReceiveBeginPlay`
  (bind (_returnvalue_roll _returnvalue_pitch) (`KismetMathLibrary.BreakRotator` (`self.K2_GetActorRotation`)))
  ;[0 0 0] Begin Play
  (`/Engine/EditorBlueprintResources/ActorMacros.Switch Has Authority`
    (:`Authority`
      (set `self.Team` (`self.GetUAVTeam` (`self.GetComponentByClass` (`GameplayStatics.GetGameState`) null)))
      (`self.K2_SetActorRotation` (`KismetMathLibrary.MakeRotator` _returnvalue_roll _returnvalue_pitch (`KismetMathLibrary.RandomFloatInRange` 0.0 360.0))))))

(fn `OnRep_bDestroyed`
  (`PrimitiveComponent.SetSimulatePhysics` (`self.StaticMesh`) true)
  (`self.SetLifeSpan` 9.0))

(fn `UserConstructionScript`)