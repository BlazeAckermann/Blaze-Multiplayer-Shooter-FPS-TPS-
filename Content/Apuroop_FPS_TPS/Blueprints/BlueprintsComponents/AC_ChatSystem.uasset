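; Actor component for multiplayer text chat with all and team channels, found on each player controller.
; The local controller creates the chat window widget at begin play, and two input actions open its entry in either mode.
; A server event loops the GameState's PlayerArray, filters by PlayerState team component for team chat, and calls each recipient's client update to display the message.
; A separate event shows server messages.
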(event `EnhancedInput|`
  (params (ActionValue :type Boolean) (ElapsedSeconds :type "Float (double-precision)") (TriggeredSeconds :type "Float (double-precision)"))
  ;[0 0 0] Input
  (:`Triggered`
    (`self.OpenChat` false)))

(event `EnhancedInput|`
  (params (ActionValue :type Boolean) (ElapsedSeconds :type "Float (double-precision)") (TriggeredSeconds :type "Float (double-precision)"))
  ;[0 0 0] Input
  (:`Triggered`
    (`self.OpenChat` true)))

(event `self.ReceiveBeginPlay`
  (bind _returnvalue (`GameplayStatics.GetPlayerController` 0))
  ;[0 0 0] Begin Play
  (if (`Controller.IsLocalController` _returnvalue)
    (bind _returnvalue_2 (`|CreateWidget` null _returnvalue))
    (bind (_output_get _output_get_2) (set `self.WB_ChatWindow` null _returnvalue_2))
    (`UserWidget.AddToViewport` _output_get_2 2)))

(event `Client_UpdateChat`
  (params (Sender :type Text) (text :type Text) (bTeamChat :type Boolean))
  (bind (_wb_chatwindow _wb_chatwindow_2) (`self.WB_ChatWindow`))
  ;[0 0 0] Update Chat
  (`/Engine/EditorBlueprintResources/StandardMacros.IsValid` _wb_chatwindow_2
    (:`Is Valid`
      (`self.UpdateChatWindow` (`/Game/Apuroop_FPS_TPS/Blueprints/BlueprintsComponents/AC_ChatSystem.ChatWindow` _wb_chatwindow_2) Sender text bTeamChat))))

(event `SendServerMessage`
  (params (Message :type Text))
  (bind (_wb_chatwindow _wb_chatwindow_2) (`self.WB_ChatWindow`))
  ;[0 0 0] Server Send message
  (`/Engine/EditorBlueprintResources/StandardMacros.IsValid` _wb_chatwindow_2
    (:`Is Valid`
      (`self.ServerMessage` (`/Game/Apuroop_FPS_TPS/Blueprints/BlueprintsComponents/AC_ChatSystem.ChatWindow` _wb_chatwindow_2) "" Message false))))

(event `Server_GetChatMessage`
  (params (TextToSend :type Text) (bTeamChat :type Boolean) (SenderPC :type "PlayerController Object Reference"))
  ;[0 0 0] Server get chat message
  (set `self.SenderText` TextToSend)
  (set `self.SenderName` (`KismetTextLibrary.Conv_StringToText` (`PlayerState.GetPlayerName` (`Controller.PlayerState` SenderPC))))
  (for _array_element (`GameStateBase.PlayerArray` (`GameplayStatics.GetGameState`))
    (bind _returnvalue (`PlayerState.GetPlayerController` _array_element))
    (`/Engine/EditorBlueprintResources/StandardMacros.IsValid` _returnvalue
      (:`Is Valid`
        (if bTeamChat
          (if (== (`self.GetTeam` (`Actor.GetComponentByClass` _array_element null)) (`self.GetTeam` (`Actor.GetComponentByClass` (`Controller.PlayerState` SenderPC) null)))
            (`self.Client_UpdateChat` (`Actor.GetComponentByClass` _returnvalue "AC_ChatSystem_C") (`self.SenderName`) (`self.SenderText`) bTeamChat :!label _label)
            (`Actor.ForceNetUpdate` (`self.GetOwner`)))
          (else
            (goto _label)))))))

(event `OpenChat`
  (params (bTeamChat :type Boolean))
  (bind _chatwindow (`/Game/Apuroop_FPS_TPS/Blueprints/BlueprintsComponents/AC_ChatSystem.ChatWindow` (`.WB_ChatWindow` (`self.WB_ChatWindow`))))
  ;[0 0 0] Open Chat
  (`self.InitChatEntry` _chatwindow bTeamChat)
  (`PlayerController.SetMouseCursorWidget` (`GameplayStatics.GetPlayerController` 0) "None" _chatwindow)
  (`Widget.SetKeyboardFocus` (`/Game/Apuroop_FPS_TPS/Blueprints/BlueprintsComponents/AC_ChatSystem.ChatEntry` _chatwindow))
  (`UserWidget.StopAllAnimations` _chatwindow))