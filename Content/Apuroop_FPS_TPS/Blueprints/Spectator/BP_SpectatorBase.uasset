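; BP_SpectatorBase is a spectator view target that shows the spectator UI and lets the player open character select to respawn.
; On becoming the local player's view target, it creates the widget, adds an input mapping and enables delayed camera lag.
; The widget signals when respawn is possible; input then opens character selection if the game state component allows respawn.
; Round end, match end or reset clears the mapping and widget.
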(event `self.K2_OnBecomeViewTarget`
  (params (PC :type "PlayerController Object Reference"))
  (bind _returnvalue (`GameplayStatics.GetPlayerController` 0))
  (bind _returnvalue_2 (`self.GetComponentByClass` (`GameplayStatics.GetGameState`) null))
  ;[0 0 0] On BecomeViewTarget
  (`/Engine/EditorBlueprintResources/StandardMacros.Can Execute Cosmetic Events`
    (:`True`
      (add `self.OnPostRound` _returnvalue_2 (delegate `DestroyWidget`))
      (add `self.OnPostMatch` _returnvalue_2 (delegate `DestroyWidget`))
      (if (== PC (`GameplayStatics.GetPlayerController` 0))
        (`|ExecutionSequence`
          (:`then_0`
            (`/Engine/EditorBlueprintResources/StandardMacros.IsValid` _returnvalue
              (:`Is Valid`
                (bind _returnvalue_3 (`|CreateWidget` null _returnvalue))
                (bind _output_get (set `self.WB_Spectator` _returnvalue_3))
                (`UserWidget.AddToViewport` _output_get 0)
                (add `self.CanRespawn` _returnvalue_3 (delegate `CanRespawn`)))))
          (:`then_1`
            (`self.EnableInput` PC)
            (`EnhancedInputSubsystemInterface.AddMappingContext` (pcsubsystem `EnhancedInputLocalPlayerSubsystem` (`GameplayStatics.GetPlayerController` 0)) null 1 (struct))
            (`KismetSystemLibrary.Delay` 1.0)
            (set `SpringArmComponent.bEnableCameraLag` true (`self.SpringArm`))))))))

(event `DestroyWidget`
  (bind _wb_spectator (`self.WB_Spectator`))
  ;[0 0 0] On BecomeViewTarget
  ;;[0 0 0] On Reset
  (`EnhancedInputSubsystemInterface.RemoveMappingContext` (pcsubsystem `EnhancedInputLocalPlayerSubsystem` (`GameplayStatics.GetPlayerController` 0)) null (struct) :!label _label)
  (`/Engine/EditorBlueprintResources/StandardMacros.IsValid` _wb_spectator
    (:`Is Valid`
      (`Widget.RemoveFromParent` _wb_spectator))))

(event `CanRespawn`
  ;[0 0 0] On BecomeViewTarget
  (set `self.bCanRespawn` true))

(event `self.K2_OnReset`
  ;[0 0 0] On BecomeViewTarget
  ;;[0 0 0] On Reset
  (goto _label))

(event `EnhancedInput|`
  (params (ActionValue :type Boolean) (ElapsedSeconds :type "Float (double-precision)") (TriggeredSeconds :type "Float (double-precision)"))
  (bind _returnvalue (`GameplayStatics.GetGameState`))
  (bind _returnvalue_2 (`self.GetComponentByClass` _returnvalue null))
  ;[0 0 0] Show Character select
  (:`Started`
    (if (or (`self.IsGameOver` _returnvalue_2) (`self.IsRoundOver` _returnvalue_2))
      (`Widget.RemoveFromParent` (`self.WB_Spectator`))
      (elif (and (`self.GetAllowRespawn` (`self.GetComponentByClass` _returnvalue null)) (`self.bCanRespawn`))
        (`EnhancedInputSubsystemInterface.RemoveMappingContext` (pcsubsystem `EnhancedInputLocalPlayerSubsystem` (`GameplayStatics.GetPlayerController` 0)) null (struct))
        (`self.Client_ShowCharacterSelectionWidget` (`self.GetComponentByClass` (`GameplayStatics.GetPlayerController` 0) null))
        (`Widget.RemoveFromParent` (`self.WB_Spectator`))))))

(event `EnhancedInput|`
  (params (ActionValue :type Boolean) (ElapsedSeconds :type "Float (double-precision)") (TriggeredSeconds :type "Float (double-precision)")))

(fn `UserConstructionScript`)