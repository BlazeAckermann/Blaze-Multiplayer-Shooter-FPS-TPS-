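; Game state Blueprint for the Capture the Flag mode that tracks both teams' flags and announces the objective.
; GetObjectives gathers the objective actors in the level and sorts them into Team 0 and Team 1 flag references.
; On player logout, any taken flag whose carrier is no longer valid gets dropped.
; Match start shows the capture message only where cosmetic events can execute.
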(event `self.GetObjectives`
  ;[0 0 0] Get Objectives
  (bind _outactors (`GameplayStatics.GetAllActorsOfClass` null))
  (set `self.Objectives` _outactors)
  (for _array_element _outactors
    (if (`KismetMathLibrary.Conv_IntToBool` (`/Game/Apuroop_FPS_TPS/Blueprints/GameModes/CaptureTheFlag/BP_CaptureTheFlag_GS.Team` _array_element))
      (set `self.FlagTeam_1` _array_element)
      (else
        (set `self.FlagTeam_0` _array_element)))))

(event `self.HandlePlayerLogout`
  (params (Controller :type "Controller Object Reference"))
  ;[0 0 0] Handle player logout
  (for _array_element (`|MakeArray` (`self.FlagTeam_1`) (`self.FlagTeam_0`))
    (`/Game/Apuroop_FPS_TPS/Blueprints/GameModes/CaptureTheFlag/BP_CaptureTheFlag_GS.Carrier` _array_element
      (:`then`)
      (:`else`
        (if (`/Game/Apuroop_FPS_TPS/Blueprints/GameModes/CaptureTheFlag/BP_CaptureTheFlag_GS.bFlagTaken` _array_element)
          (`self.DropFlag` _array_element))))))

(event `self.MatchStateSystem.OnStartMatch`
  (`/Engine/EditorBlueprintResources/StandardMacros.Can Execute Cosmetic Events`
    (:`True`
      (`self.ShowObjectiveMessage` "Capture the enemy flag"))))

(fn `UserConstructionScript`
  (`parent.UserConstructionScript`))