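; Free-for-all game mode that puts each starting player on their own team, identified by a random number.
; On HandleStartingNewPlayer, it sets the team on a component of the player's PlayerState, using the value from GetUniqueTeam.
; GetUniqueTeam gathers the teams already held across the GameState's PlayerArray, then re-rolls random IDs from 2 to 255 until one is unused.
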(event `self.ReceiveBeginPlay`
  ;[0 0 0] Begin Play
  (`parent.ReceiveBeginPlay`))

(event `self.HandleStartingNewPlayer`
  (params (NewPlayer :type "PlayerController Object Reference"))
  ;[0 0 0] Handle Starting New Player
  (bind _team (`self.GetUniqueTeam`))
  (`self.SetTeam` (`self.GetComponentByClass` (`Controller.PlayerState` NewPlayer) null) _team))

(fn `GetUniqueTeam`
  (returns (Team :type Integer))
  (locals (UsedTeams :type "Array of Integer") (PossibleTeam :type Integer))
  (`KismetArrayLibrary.Array_Clear` (`local.UsedTeams`))
  (for _array_element (`GameStateBase.PlayerArray` (`GameplayStatics.GetGameState`))
    (bind _returnvalue (`self.GetComponentByClass` _array_element null))
    (`/Engine/EditorBlueprintResources/StandardMacros.IsValid` _returnvalue
      (:`Is Valid`
        (`KismetArrayLibrary.Array_AddUnique` (`local.UsedTeams`) (`self.GetTeam` _returnvalue)))))
  (set `local.PossibleTeam` (`KismetMathLibrary.RandomIntegerInRange` 2 255) :!label _label)
  (if (`KismetArrayLibrary.Array_Contains` (`local.UsedTeams`) (`local.PossibleTeam`))
    (goto _label)
    (else
      (return (`local.PossibleTeam`)))))

(fn `UserConstructionScript`
  (`parent.UserConstructionScript`))