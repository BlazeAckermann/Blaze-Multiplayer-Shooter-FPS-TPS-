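; BP_Claymore is a team-aware, server-authoritative claymore mine that its owner can pick back up as lethal ammo by interacting.
; It explodes when a character from another team enters its trigger box or when damage depletes its health component, awarding score to enemies who destroy it.
; Explosion applies radial damage, multicasts particle, sound and camera shake effects, then hides the mesh and expires after a short lifespan.
; Net dormancy is woken on trigger or damage, and a replicated destroyed flag updates clients.
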(event `self.K2_OnReset`
  (`self.K2_DestroyActor`))

(event `self.ReceiveBeginPlay`
  (bind _instigator (`self.Instigator`))
  ;[0 0 0] Begin play
  (`/Engine/EditorBlueprintResources/ActorMacros.Switch Has Authority`
    (:`Authority`
      (set `self.InstigatorController` (`self.GetInstigatorController` _instigator))
      (set `self.Team` (`self.GetTeam` (`self.GetComponentByClass` (`Pawn.PlayerState` _instigator) null)))
      (`self.FlushNetDormancy`))))

(event `self.ReceiveAnyDamage`
  (params (Damage :type "Float (single-precision)") (DamageType :type "DamageType Object Reference") (InstigatedBy :type "Controller Object Reference") (DamageCauser :type "Actor Object Reference"))
  (bind _bp_healthcomponent (`self.BP_HealthComponent`))
  (bind _playerstate (`Controller.PlayerState` InstigatedBy))
  ;[0 0 0] Any Damage
  (if (not (`self.bDestroyed`))
    (message `/Game/Apuroop_FPS_TPS/Blueprints/Explosives/BP_Claymore.ShowHitMarker` (`Controller.K2_GetPawn` InstigatedBy) false)
    (`self.SetNetDormancy` "DORM_Awake")
    (`self.HandleDamage` _bp_healthcomponent Damage)
    (if (`self.IsDead` _bp_healthcomponent)
      (if (!= (`self.GetTeam` (`self.GetComponentByClass` _playerstate null)) (`self.Team`))
        (message `/Game/Apuroop_FPS_TPS/Blueprints/Explosives/BP_Claymore.AddScoreToPlayer` _playerstate 20.0 0))
      (`self.Explode` InstigatedBy))))

(event `self.Box.OnComponentBeginOverlap`
  (params (OverlappedComponent :type "PrimitiveComponent Object Reference") (OtherActor :type "Actor Object Reference") (OtherComp :type "PrimitiveComponent Object Reference") (OtherBodyIndex :type Integer) (bFromSweep :type Boolean) (SweepResult :type "HitResult Structure (by ref)"))
  ;[0 0 0] On overlap
  (bind _ascharacter (cast `Character` OtherActor))
  (`/Engine/EditorBlueprintResources/ActorMacros.Switch Has Authority`
    (:`Authority`
      (if (not (`self.bDestroyed`))
        (if (not (== (`self.GetTeam` (`self.GetComponentByClass` (`Pawn.PlayerState` _ascharacter) null)) (`self.Team`)))
          (`self.SetNetDormancy` "DORM_Awake")
          (`self.Explode` (`self.InstigatorController`)))))))

(event `Explode`
  (params (Instigator :type "Controller Object Reference"))
  (bind (_returnvalue_x _returnvalue_y _returnvalue_z) (`KismetMathLibrary.BreakVector` (`SceneComponent.K2_GetComponentLocation` (`self.Box`))))
  ;[0 0 0] Explode
  (`KismetSystemLibrary.Delay` 0.0) ; Next Frame
  (set `self.bDestroyed` true)
  (`GameplayStatics.ApplyRadialDamage` :`BaseDamage` 500.0 :`Origin` (`KismetMathLibrary.MakeVector` _returnvalue_x _returnvalue_y _returnvalue_z) :`DamageRadius` (`self.Radius`) :`DamageCauser` self :`InstigatedByController` Instigator :`DamagePreventionChannel` "ECC_WorldDynamic")
  (`self.MulticastPlayCosmeticEffects`)
  (`SceneComponent.SetVisibility` (`self.Mesh`) false false)
  (`self.SetLifeSpan` 3.0)
  (`ActorComponent.K2_DestroyComponent` (`self.ChildActor`))
  (`self.ForceNetUpdate`))

(event `MulticastPlayCosmeticEffects`
  (bind _radius (`self.Radius`))
  (bind _returnvalue (`self.K2_GetActorLocation` self))
  ;[0 0 0] Play Cosmetic Effects
  (`/Engine/EditorBlueprintResources/StandardMacros.Can Execute Cosmetic Events`
    (:`True`
      (`GameplayStatics.SpawnEmitterAtLocation` null _returnvalue (struct) (5.0 5.0 5.0))
      (`GameplayStatics.PlaySoundAtLocation` null _returnvalue (struct) 0.5 1.0 0.0 null null null null)
      (`GameplayStatics.PlayWorldCameraShake` null _returnvalue (* _radius 2.0) (* _radius 3.0)))))

(event `self.Interact`
  (params (InstigatorPawn :type "Pawn Object Reference"))
  ;[0 0 0] On Interact
  (if (and (== (`Pawn.GetController` InstigatorPawn) (`self.InstigatorController`)) (not (`self.bDestroyed`)))
    (`self.AddLethalAmmo` (`self.GetComponentByClass` InstigatorPawn null))
    (`self.K2_DestroyActor`)))

(fn `OnRep_bDestroyed`
  (bind _mesh (`self.Mesh`))
  (`SceneComponent.SetVisibility` _mesh false false)
  (`PrimitiveComponent.SetCollisionEnabled` _mesh "NoCollision"))

(fn `UserConstructionScript`)